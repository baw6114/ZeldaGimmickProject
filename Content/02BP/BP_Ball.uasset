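; BP_Ball is a physics ball that can be grabbed, thrown and set off like a bomb.
; Grab turns off physics simulation and collision on the Sphere, and Throw restores both before applying the given vector as a velocity-change impulse, which ignores mass.
; Bomb activates a particle system, fires a radial force impulse and prints a debug string, without destroying the ball.
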(event `/Game/02BP/BI_GripObject.Grab`
  (bind _sphere (`self.Sphere`))
  (`PrimitiveComponent.SetSimulatePhysics` _sphere false)
  (`PrimitiveComponent.SetCollisionEnabled` _sphere "NoCollision"))

(event `/Game/02BP/BI_GripObject.Throw`
  (params (Location :type "Vector Structure"))
  (bind _sphere (`self.Sphere`))
  (`PrimitiveComponent.SetSimulatePhysics` _sphere true)
  (`PrimitiveComponent.SetCollisionEnabled` _sphere "QueryAndPhysics")
  (`PrimitiveComponent.AddImpulse` _sphere Location "None" true))

(event `/Game/02BP/BI_Bomber.Bomb`
  (`ActorComponent.Activate` (`self.ParticleSystem`) true)
  (`RadialForceComponent.FireImpulse` (`self.RadialForce`))
  (`KismetSystemLibrary.PrintString` "Hello"))

(fn `UserConstructionScript`)